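; Ocean controller Blueprint that sets water color and swaps wave assets on the level's WaterBodyOcean.
; BeginPlay writes a green WaterColor to the MPC_OceanParams material parameter collection and caches the ocean actor.
; The T key flip-flops between calm (OndasCalmas) and storm (OndasTempestade) waves.
; Tick is also wired to the storm call, so storm waves are reapplied every frame, overriding the calm toggle.
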(event EventBeginPlay
  (Rendering|Material|SetVectorParameterValue "/Game/MPC_OceanParams.MPC_OceanParams" "WaterColor" (Utilities|Struct|MakeLinearColor 0.0 5e+01 0.0 1.0) :!class /Script/Engine.KismetMaterialLibrary)
  (bind _returnvalue (Actor|GetActorOfClass "/Script/Water.WaterBodyOcean"))
  (Variables|Default|SetOceanActor _returnvalue))

(event EventTick
  (params (DeltaSeconds :type Float%20%28single-precision%29))
  (Class|WaterBody|SetWaterWaves (Variables|Default|GetOceanActor) (Variables|Default|GetOndasTempestade)))

(event Input|KeyboardEvents|T
  (params (Key :type Key%20Structure :default "None"))
  (:Pressed
    (Utilities|FlowControl|FlipFlop
      (:A
        (Class|WaterBody|SetWaterWaves (Variables|Default|GetOceanActor) (Variables|Default|GetOndasCalmas)))
      (:B
        (Class|WaterBody|SetWaterWaves (Variables|Default|GetOceanActor) (Variables|Default|GetOndasTempestade))))))

(fn ConstructionScript)