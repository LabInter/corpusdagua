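; BP_OSC drives rain and smoke effects from people-tracking OSC messages received through BP_OSCManager.
; On BeginPlay it finds a Niagara rain actor and a smoke Emitter, then binds to the manager; Tick keeps the rain above the camera.
; MessageReceive routes by address: people count scales RainIntensity, and per-person coordinates are range-mapped to move the single smoke actor.
; Wildcard-matched left/right hand open and closed messages only print debug text.
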(event Custom|MessageReceive
  (params (Message :type String) (OSCMessage :type OSC%20Message%20Structure))
  (bind _rainactor (Variables|Default|GetRainActor))
  (bind _returnvalue (Class|OSCManager|GetOSCMessageAddress OSCMessage))
  (bind _returnvalue_2 (Class|OSCManager|GetOSCAddressFullPath _returnvalue))
  (Utilities|FlowControl|Sequence
    (:then_0
      (if (Utilities|Enum|Equal(Enum) _returnvalue_2 "/people/count")
        (Utilities|IsValid (Variables|Default|GetRainActor)
          (:Is%20Valid
            (bind _value (Class|OSCManager|GetFloat OSCMessage))
            (Niagara|SetNiagaraVariable(Float) (Variables|/Script/Niagara.NiagaraActor|GetNiagaraComponent _rainactor) "RainIntensity" (* _value 1.5e+03))
            (Development|PrintString (Utilities|GetDisplayName _rainactor) false false)))))
    (:then_1
      (if (Class|KismetStringLibrary|MatchesWildcard _returnvalue_2 "/people/*/mao_esquerda_aberta" "IgnoreCase")
        (Class|OSCManager|GetBool OSCMessage)
        (Development|PrintText "Mão esquerda ABERTA" false false)))
    (:then_2
      (if (Class|KismetStringLibrary|MatchesWildcard _returnvalue_2 "/people/*/mao_esquerda_fechada" "IgnoreCase")
        (Class|OSCManager|GetBool OSCMessage)
        (Development|PrintText "Mão esquerda FECHADA" false false)))
    (:then_3
      (if (Class|KismetStringLibrary|MatchesWildcard _returnvalue_2 "/people/*/mao_direita_aberta" "IgnoreCase")
        (Class|OSCManager|GetBool OSCMessage)
        (Development|PrintText "Mão direita ABERTA" false false)))
    (:then_4
      (if (Class|KismetStringLibrary|MatchesWildcard _returnvalue_2 "/people/*/mao_direita_fechada" "IgnoreCase")
        (Class|OSCManager|GetBool OSCMessage)
        (Development|PrintText "Mão direita FECHADA" false false)))
    (:then_5
      (if (Class|KismetStringLibrary|MatchesWildcard _returnvalue_2 "/people/?" "IgnoreCase")
        (Utilities|FlowControl|Sequence
          (:then_0
            (bind _value_2 (Class|OSCManager|GetFloat OSCMessage)))
          (:then_1
            (bind _value_3 (Class|OSCManager|GetFloat OSCMessage 1))))
        (Transformation|SetActorLocation (Variables|Default|GetSmokeActor) (Math|Vector|MakeVector (Math|Float|MapRangeClamped _value_2 -1.0 1.0 -2.52e+04 2.52e+04) (Math|Float|MapRangeClamped _value_3 -1.0 1.0 -2.52e+04 2.52e+04) 0.0) false false)
        (Development|PrintText (Utilities|Text|ToText(String) (Math|Vector|MakeVector (Math|Float|MapRangeClamped _value_2 -1.0 1.0 -2.52e+04 2.52e+04) (Math|Float|MapRangeClamped _value_3 -1.0 1.0 -2.52e+04 2.52e+04) 0.0)))
        (Variables|Default|Setposition (Math|Vector|MakeVector (Math|Float|MapRangeClamped _value_2 -1.0 1.0 -2.52e+04 2.52e+04) (Math|Float|MapRangeClamped _value_3 -1.0 1.0 -2.52e+04 2.52e+04) 0.0))))))

(event EventBeginPlay
  (bind _returnvalue (Actor|GetActorOfClass "/Script/Engine.Emitter"))
  (bind _returnvalue_2 (Actor|GetActorOfClass "/Script/Niagara.NiagaraActor"))
  (Utilities|FlowControl|Sequence
    (:then_0
      (bind _output_get (Variables|Default|SetRainActor _returnvalue_2))
      (Development|PrintString (Utilities|GetDisplayName _output_get) false false)
      (Variables|Default|SetOSCServer (Variables|Default|GetOSCServer))
      (bind _returnvalue_3 (Actor|GetActorOfClass "/Game/BP_OSCManager.BP_OSCManager_C"))
      (EventDispatchers|BindEventtoOnOSCMessageReceived _returnvalue_3 (EventDispatchers|CreateEvent :!event Custom|MessageReceive)))
    (:then_1
      (bind _output_get_2 (Variables|Default|SetSmokeActor _returnvalue))
      (Development|PrintString (Utilities|GetDisplayName _output_get_2))
      (Variables|Default|SetOSCServer (Variables|Default|GetOSCServer))
      (bind _returnvalue_4 (Actor|GetActorOfClass "/Game/BP_OSCManager.BP_OSCManager_C"))
      (EventDispatchers|BindEventtoOnOSCMessageReceived _returnvalue_4 (EventDispatchers|CreateEvent :!event Custom|MessageReceive)))))

(event EventTick
  (params (DeltaSeconds :type Float%20%28single-precision%29))
  (bind _rainactor (Variables|Default|GetRainActor))
  (Utilities|IsValid _rainactor
    (:Is%20Valid
      (Transformation|SetActorLocation _rainactor (+ (Camera|GetCameraLocation (Game|GetPlayerCameraManager 0)) "0.000000,0.000000,1000.000000") false true))))

(fn ConstructionScript)